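; BP_Phase2Gate is the gate for boss phase 2.5, opening and closing once on a fixed timer.
; BeginPlay waits about 22 seconds, slides SMHallDoorL to the Open component's relative location, pauses briefly, then slides it to Close.
; Both moves use MoveComponentTo with ease in and out over MovingTime, driven only by delays rather than boss state.
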(event `self.ReceiveBeginPlay`
  ;[1 1 1] 보스 2.5 페이즈 게이트 개폐
  (`KismetSystemLibrary.Delay` 22.0)
  (`KismetSystemLibrary.MoveComponentTo` (`self.SM_Hall_Door_L`) (`SceneComponent.RelativeLocation` (`self.Open`)) (struct) true true (`self.MovingTime`))
  (`KismetSystemLibrary.Delay` 2.0)
  (`KismetSystemLibrary.MoveComponentTo` (`self.SM_Hall_Door_L`) (`SceneComponent.RelativeLocation` (`self.Close`)) (struct) true true (`self.MovingTime`)))

(fn `UserConstructionScript`)