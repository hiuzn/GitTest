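; Sliding gate for the boss phase 2.5 area that the player opens with E while holding a cardkey.
; The box overlap toggles input and a prompt widget; without the cardkey, E prints a warning and plays an error sound.
; With it, a one-shot path plays a sound, waits, then eases the door to the Open marker's position.
; CloseGate moves it to the Close marker, while OpenGate is an empty stub.
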(event `self.Box.OnComponentBeginOverlap`
  (params (OverlappedComponent :type "PrimitiveComponent Object Reference") (OtherActor :type "Actor Object Reference") (OtherComp :type "PrimitiveComponent Object Reference") (OtherBodyIndex :type Integer) (bFromSweep :type Boolean) (SweepResult :type "HitResult Structure (by ref)"))
  (`self.EnableInput` (`GameplayStatics.GetPlayerController` 0))
  (`SceneComponent.SetVisibility` (`self.Widget`) true false))

(event `self.Box.OnComponentEndOverlap`
  (params (OverlappedComponent :type "PrimitiveComponent Object Reference") (OtherActor :type "Actor Object Reference") (OtherComp :type "PrimitiveComponent Object Reference") (OtherBodyIndex :type Integer))
  (`self.DisableInput` (`GameplayStatics.GetPlayerController` 0))
  (`SceneComponent.SetVisibility` (`self.Widget`) false false))

(event `Key|E`
  (params (Key :type "Key Structure"))
  (:`Pressed`
    (bind _asbp_third_person_character (cast `/Game/ThirdPerson/Blueprints/BP_ThirdPersonCharacter` (`GameplayStatics.GetPlayerCharacter` 0)))
    (if (`/Game/ThirdPerson/Blueprints/BP_ThirdPersonCharacter.HasCardkey` _asbp_third_person_character)
      (`/Engine/EditorBlueprintResources/StandardMacros.DoOnce` false
        (:`Completed`
          (`/Engine/EditorBlueprintResources/StandardMacros.FlipFlop`
            (:`A`
              (`GameplayStatics.PlaySoundAtLocation` "/Game/BluePrints/Door/VaccinDoor_Open.VaccinDoor_Open" (`self.K2_GetActorLocation`) (struct) 1.0 1.0 0.0 null null null null)
              (`KismetSystemLibrary.Delay` 1.0)
              (`KismetSystemLibrary.MoveComponentTo` (`self.SM_Hall_Door_L`) (`SceneComponent.RelativeLocation` (`self.Open`)) (struct) true true (`self.MovingTime`))))))
      (else
        (`KismetSystemLibrary.PrintString` "카드키를 챙기세요!!!")
        (`GameplayStatics.PlaySoundAtLocation` "/Game/Sounds/wrong-answer-error.wrong-answer-error" (`self.K2_GetActorLocation`) (struct) 1.0 1.0 0.0 null null null null)))))

(event `OpenGate`
  ;[1 1 1] 보스 2.5 페이즈 게이트 개폐
)

(event `CloseGate`
  ;[1 1 1] 보스 2.5 페이즈 게이트 개폐
  (`KismetSystemLibrary.MoveComponentTo` (`self.SM_Hall_Door_L`) (`SceneComponent.RelativeLocation` (`self.Close`)) (struct) true true (`self.MovingTime`)))

(fn `UserConstructionScript`)