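; BP_BossStartZone is the boss arena's start area, which opens up through moving set pieces when its Active event is called.
; A Sequence eases the floor down and the ceiling up together, using MoveComponentTo toward marker component positions.
; After the floor finishes, it triggers MovingFloors on BossFloors, waits, then moves a wall to the raised glass position.
; Separate robot arm moves are left unconnected and never run.
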(event `Active`
  (`|ExecutionSequence`
    (:`then_0`
      ;[1 1 1] 바닥, 바닥 로봇팔 아래로 이동
      (`KismetSystemLibrary.MoveComponentTo` (`self.StageFloor_1`) (`SceneComponent.RelativeLocation` (`self.PosDown`)) (struct) true true (`self.MovingTime`))
      (`/Game/LJK_Assets/BP_BossFloors.MovingFloors` (`self.BossFloors`))
      (`KismetSystemLibrary.Delay` 5.0)
      (`KismetSystemLibrary.MoveComponentTo` (`self.SM_Wall_C`) (`SceneComponent.RelativeLocation` (`self.PosUpGlass`)) (struct) true true 3.0))
    (:`then_1`
      ;[1 1 1] 위쪽 천장, 로봇팔 위로 이동
      (`KismetSystemLibrary.MoveComponentTo` (`self.SM_Ceiling_Main`) (`SceneComponent.RelativeLocation` (`self.PosUpCeiling`)) (struct) true true (`self.MovingTime`)))))

(fn `UserConstructionScript`)