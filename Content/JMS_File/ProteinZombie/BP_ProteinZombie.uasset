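; Protein zombie enemy that chases the player from BeginPlay, speeds up when PawnSensing sees a pawn, and attacks in melee.
; On arrival it randomly plays a punch or swipe montage with a matching player camera-boom call, then resumes the chase.
; Montage notifies apply damage through a sphere overlap at an arrow component.
; Nonlethal hits set its capsule to overlap pawns; zero health stops movement and plays a dying montage.
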(event `self.ReceiveBeginPlay`
  (`self.RunToPlayer`))

(event `self.PawnSensing.OnSeePawn`
  (params (Pawn :type "Pawn Object Reference"))
  ;[1 1 1] 인지 범위 안에 들어오면 속도 up
  (set `CharacterMovementComponent.MaxWalkSpeed` 300.0 (`self.CharacterMovement`)))

(event `RunToPlayer`
  ;[1 1 1] 플레이어한테 다가가기
  (if (not (`self.IsDead`))
    (`|AIMoveTo` self (0.0 0.0 0.0) (`GameplayStatics.GetPlayerController` 0) 100.0
      (:`OnSuccess`
        (`self.AttackPlayer`))
      (:`OnFail`
        (`self.RuntoPlayer`)))))

(event `AttackPlayer`
  (bind _returnvalue (`GameplayStatics.GetPlayerCharacter` 0))
  (bind _mesh (`self.Mesh`))
  ;[1 1 1] 플레이어 공격 애니메이션
  (bind _output_get (set `self.Protein_Attack` (cast `/Game/JMS_File/ProteinZombie/E_ProteinAttack` (`KismetMathLibrary.Conv_IntToByte` (`KismetMathLibrary.RandomInteger` 2)))))
  (switch `/Game/JMS_File/ProteinZombie/E_ProteinAttack` _output_get
    (:`NewEnumerator0`
      (bind _asbp_third_person_character (cast `/Game/ThirdPerson/Blueprints/BP_ThirdPersonCharacter` _returnvalue))
      (`/Game/ThirdPerson/Blueprints/BP_ThirdPersonCharacter.Camera Boom Punch` _asbp_third_person_character)
      (`|PlayMontage` _mesh "/Game/JMS_File/ProteinZombie/Animations/Attack/Mutant_Punch_Montage.Mutant_Punch_Montage"
        (:`OnCompleted`
          (`self.RunToPlayer` :!label _label))
        (:`OnNotifyBegin`
          ;[1 1 1] 사거리 안에 들어오면 데미지 입음
          (bind (_outactors _returnvalue_2) (`KismetSystemLibrary.SphereOverlapActors` (`SceneComponent.K2_GetComponentLocation` (`self.Arrow1`)) 200.0 (`|MakeArray` "ObjectTypeQuery3" :!type "EObjectTypeQuery Enum") "/Game/ThirdPerson/Blueprints/BP_ThirdPersonCharacter.BP_ThirdPersonCharacter_C" (`|MakeArray` self :!type "Actor Object Reference") :!label _label_2))
          (if _returnvalue_2
            (for _array_element _outactors
              (`GameplayStatics.ApplyDamage` _array_element 20.0 (`self.GetController`) self "/Script/Engine.DamageType"))))))
    (:`NewEnumerator1`
      (bind _asbp_third_person_character_2 (cast `/Game/ThirdPerson/Blueprints/BP_ThirdPersonCharacter` _returnvalue))
      (`/Game/ThirdPerson/Blueprints/BP_ThirdPersonCharacter.Camera Boom Swiping` _asbp_third_person_character_2)
      (`|PlayMontage` _mesh "/Game/JMS_File/ProteinZombie/Animations/Attack/mutant_swiping_Montage.mutant_swiping_Montage"
        (:`OnCompleted`
          (goto _label))
        (:`OnNotifyBegin`
          (goto _label_2))))))

(event `self.ReceiveAnyDamage`
  (params (Damage :type "Float (single-precision)") (DamageType :type "DamageType Object Reference") (InstigatedBy :type "Controller Object Reference") (DamageCauser :type "Actor Object Reference"))
  ;[1 1 1] 프로틴 좀비가 데미지 입는 노드
  (if (`self.IsDead`)
    _
    (elif (<= (`self.Health`) 0.0)
      (`self.Death`)
      (else
        (bind _output_get (set `self.Health` (- (`self.Health`) Damage)))
        (if (<= _output_get 0.0)
          (`self.Death`)
          (else
            (`PrimitiveComponent.SetCollisionResponseToChannel` (`self.CapsuleComponent`) "ECC_Pawn" "ECR_Overlap")))))))

(event `Death`
  ;[1 1 1] 프로틴 좀비 사망
  (set `self.IsDead` true)
  (`MovementComponent.StopMovementImmediately` (`self.CharacterMovement`))
  (`|PlayMontage` (`self.Mesh`) "/Game/JMS_File/ProteinZombie/Animations/mutant_dying_Montage.mutant_dying_Montage"))

(fn `UserConstructionScript`)