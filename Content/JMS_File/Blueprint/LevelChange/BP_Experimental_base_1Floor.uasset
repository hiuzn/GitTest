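; BP_Experimental_base_1Floor is a trigger actor that moves the player to the Experimental_base_1Floor level when they stay inside its Box.
; Overlapping the Box with BP_ThirdPersonCharacter starts a three-second delay, then shows the WB_fade widget with its fade animation and opens the level half a second later.
; An In flag, cleared on end overlap, is rechecked after each delay to cancel the transition if it is false.
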(event `self.Box.OnComponentBeginOverlap`
  (params (OverlappedComponent :type "PrimitiveComponent Object Reference") (OtherActor :type "Actor Object Reference") (OtherComp :type "PrimitiveComponent Object Reference") (OtherBodyIndex :type Integer) (bFromSweep :type Boolean) (SweepResult :type "HitResult Structure (by ref)"))
  (set `self.In` true)
  (cast `/Game/ThirdPerson/Blueprints/BP_ThirdPersonCharacter` OtherActor)
  (`KismetSystemLibrary.Delay` 3.0)
  (if (`self.In`)
    (bind _returnvalue (`|CreateWidget` "/Game/JMS_File/Blueprint/WB_fade.WB_fade_C"))
    (`UserWidget.AddToViewport` _returnvalue 0)
    (`/Game/JMS_File/Blueprint/WB_fade.FadeAnim` _returnvalue)
    (`KismetSystemLibrary.Delay` 0.5)
    (if (`self.In`)
      (`GameplayStatics.OpenLevel` "Experimental_base_1Floor"))))

(event `self.Box.OnComponentEndOverlap`
  (params (OverlappedComponent :type "PrimitiveComponent Object Reference") (OtherActor :type "Actor Object Reference") (OtherComp :type "PrimitiveComponent Object Reference") (OtherBodyIndex :type Integer))
  (set `self.In` false))

(fn `UserConstructionScript`)