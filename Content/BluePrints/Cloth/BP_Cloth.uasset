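; BP_Cloth is a clothing pickup that changes the player character's skeletal mesh to SK_Man_Full_04.
; Sphere overlap with the player shows an interact widget and enables input, and ending overlap reverses both.
; Pressing E while IsRead is false swaps the mesh, hides the widget and destroys the actor after a short delay.
; An uncalled PickUpItem function plays a sound and sets the character's HasLaptop flag, apparently left from another item.
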(event `self.Sphere.OnComponentBeginOverlap`
  (params (OverlappedComponent :type "PrimitiveComponent Object Reference") (OtherActor :type "Actor Object Reference") (OtherComp :type "PrimitiveComponent Object Reference") (OtherBodyIndex :type Integer) (bFromSweep :type Boolean) (SweepResult :type "HitResult Structure (by ref)"))
  (if (== (`GameplayStatics.GetPlayerCharacter` 0) OtherActor)
    (`SceneComponent.SetVisibility` (`self.Interact Widget`) true false)
    (`self.EnableInput` (`GameplayStatics.GetPlayerController` 0))))

(event `self.Sphere.OnComponentEndOverlap`
  (params (OverlappedComponent :type "PrimitiveComponent Object Reference") (OtherActor :type "Actor Object Reference") (OtherComp :type "PrimitiveComponent Object Reference") (OtherBodyIndex :type Integer))
  (`SceneComponent.SetVisibility` (`self.Interact Widget`) false false)
  (`self.DisableInput` (`GameplayStatics.GetPlayerController` 0)))

(event `Key|E`
  (params (Key :type "Key Structure"))
  (:`Pressed`
    (if (not (`self.IsRead?`))
      (`SkeletalMeshComponent.SetSkeletalMeshAsset` (`Character.Mesh` (`GameplayStatics.GetPlayerCharacter` 0)) "/Game/ThirdPerson/Man/Mesh/Full/SK_Man_Full_04.SK_Man_Full_04")
      (`SceneComponent.SetVisibility` (`self.Interact Widget`) false false)
      (`self.K2_DestroyActor`))))

(event `Destroy Actor`
  (`KismetSystemLibrary.Delay` 0.1)
  (`self.K2_DestroyActor`))

(fn `Pick Up Item`
  (returns (item :type String))
  (`KismetSystemLibrary.PrintString` "Item Picked!!")
  (`self.Destroy Actor`)
  (`GameplayStatics.PlaySoundAtLocation` "/Game/BluePrints/Laptop/get_things.get_things" (`self.K2_GetActorLocation`) (struct) 1.0 1.0 0.0 null null null null)
  (bind _asbp_third_person_character (cast `/Game/ThirdPerson/Blueprints/BP_ThirdPersonCharacter` (`GameplayStatics.GetPlayerCharacter` 0)))
  (set `/Game/ThirdPerson/Blueprints/BP_ThirdPersonCharacter.HasLaptop` true _asbp_third_person_character)
  (return (`self.item`)))

(fn `UserConstructionScript`)