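; BP_Door is a two-panel sliding door that the player toggles with E while inside its trigger box.
; Box overlap enables input and shows a widget, and leaving reverses both.
; E plays an elevator door sound and flip-flops between playing the timeline after a short delay and reversing it.
; The timeline lerps both panels' relative locations, and a Delay on its update reverses it automatically, independently of the FlipFlop state.
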(event `self.Box.OnComponentBeginOverlap`
  (params (OverlappedComponent :type "PrimitiveComponent Object Reference") (OtherActor :type "Actor Object Reference") (OtherComp :type "PrimitiveComponent Object Reference") (OtherBodyIndex :type Integer) (bFromSweep :type Boolean) (SweepResult :type "HitResult Structure (by ref)"))
  (`self.EnableInput` (`GameplayStatics.GetPlayerController` 0))
  (`SceneComponent.SetVisibility` (`self.Widget`) true false))

(event `self.Box.OnComponentEndOverlap`
  (params (OverlappedComponent :type "PrimitiveComponent Object Reference") (OtherActor :type "Actor Object Reference") (OtherComp :type "PrimitiveComponent Object Reference") (OtherBodyIndex :type Integer))
  (`self.DisableInput` (`GameplayStatics.GetPlayerController` 0))
  (`SceneComponent.SetVisibility` (`self.Widget`) false false))

(event `Key|E`
  (params (Key :type "Key Structure"))
  (:`Pressed`
    (`GameplayStatics.PlaySoundAtLocation` "/Game/BluePrints/Door/elevator-door-opens-and-closes.elevator-door-opens-and-closes" (`self.K2_GetActorLocation`) (struct) 1.0 1.0 0.0 null null null null)
    (`/Engine/EditorBlueprintResources/StandardMacros.FlipFlop`
      (:`A`
        (`KismetSystemLibrary.Delay` 1.0)
        (bind (_direction _slide) (`Timeline|타임라인` :!label _label)
          (:`Update`
            (`SceneComponent.K2_SetRelativeLocation` (`self.DoorB`) (`KismetMathLibrary.VLerp` (`self.CurrentDoorB`) (`self.NewDoorB`) _slide) false false)
            (`SceneComponent.K2_SetRelativeLocation` (`self.DoorA`) (`KismetMathLibrary.VLerp` (`self.CurrentDoorA`) (`self.NewDoorA`) _slide) false false)
            (`KismetSystemLibrary.Delay` 5.0)
            (goto _label :!via `Reverse`))))
      (:`B`
        (goto _label :!via `Reverse`)))))

(fn `UserConstructionScript`)