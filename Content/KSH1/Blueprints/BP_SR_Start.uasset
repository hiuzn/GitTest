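; BP_SR_Start is a shoot-to-start actor that sends the player to the Laboratory1 level.
; Entering its Box volume hides the Widget component and leaving shows it again, with no filter on the overlapping actor.
; When IsActive is true, a BP_Bullet_Player overlapping the Widget hides it, then plays a WB_fade screen fade after a delay and opens the level shortly afterwards.
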(event `self.Box.OnComponentBeginOverlap`
  (params (OverlappedComponent :type "PrimitiveComponent Object Reference") (OtherActor :type "Actor Object Reference") (OtherComp :type "PrimitiveComponent Object Reference") (OtherBodyIndex :type Integer) (bFromSweep :type Boolean) (SweepResult :type "HitResult Structure (by ref)"))
  (`SceneComponent.SetVisibility` (`self.Widget`) false false))

(event `self.Box.OnComponentEndOverlap`
  (params (OverlappedComponent :type "PrimitiveComponent Object Reference") (OtherActor :type "Actor Object Reference") (OtherComp :type "PrimitiveComponent Object Reference") (OtherBodyIndex :type Integer))
  (`SceneComponent.SetVisibility` (`self.Widget`) true false))

(event `self.Widget.OnComponentBeginOverlap`
  (params (OverlappedComponent :type "PrimitiveComponent Object Reference") (OtherActor :type "Actor Object Reference") (OtherComp :type "PrimitiveComponent Object Reference") (OtherBodyIndex :type Integer) (bFromSweep :type Boolean) (SweepResult :type "HitResult Structure (by ref)"))
  ;[1 1 1] 위젯 눌러서 실험기지로 이동
  (if (`self.IsActive`)
    (cast `/Game/KSH1/Blueprints/BP_Bullet_Player` OtherActor)
    (`SceneComponent.SetVisibility` (`self.Widget`) false false)
    (`KismetSystemLibrary.Delay` 1.0)
    (bind _returnvalue (`|CreateWidget` "/Game/JMS_File/Blueprint/WB_fade.WB_fade_C"))
    (`UserWidget.AddToViewport` _returnvalue 0)
    (`/Game/JMS_File/Blueprint/WB_fade.FadeAnim` _returnvalue)
    (`KismetSystemLibrary.Delay` 0.5)
    (`GameplayStatics.OpenLevel` "Laboratory1")))

(fn `UserConstructionScript`)