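; BP_Target is a damageable shooting target that plays a death animation at zero health and revives after a reset delay.
; AnyDamage lowers and prints Health, then on death calls UpdateScore, returns SMFloorA1 to PosA and starts PlayTargetDrop, which restores health and idle animation.
; MoveComponentTo shuttles the floor mesh between PosA and PosB, with OnActive entering that loop.
; UpdateScore is empty, leaving the player AddScore logic disconnected.
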(event `self.ReceiveAnyDamage`
  (params (Damage :type "Float (single-precision)") (DamageType :type "DamageType Object Reference") (InstigatedBy :type "Controller Object Reference") (DamageCauser :type "Actor Object Reference"))
  (if (> (`self.Health`) 0.0)
    (set `self.Health` (- (`self.Health`) Damage))
    (`KismetSystemLibrary.PrintString` (`KismetStringLibrary.Conv_DoubleToString` (`self.Health`)) true true (struct :`R` 1.0 :`G` 0.950883 :`B` 0.066792 :`A` 1.0) 3.0)
    (if (<= (`self.Health`) 0.0)
      (`SkeletalMeshComponent.PlayAnimation` (`self.Target`) "/Game/AnimStarterPack/Death_1.Death_1" false)
      (`KismetSystemLibrary.Delay` 1.0)
      (`self.UpdateScore` 1)
      (`SceneComponent.K2_SetWorldLocation` (`self.SM_Floor_A1`) (`SceneComponent.K2_GetComponentLocation` (`self.PosA`)) false true)
      (`KismetSystemLibrary.MoveComponentTo` (`self.SM_Floor_A1`) (`SceneComponent.RelativeLocation` (`self.PosA`)) (struct) false false (`self.ResetMovingTime`))
      (`SkeletalMeshComponent.Stop` (`self.Target`))
      (`self.PlayTargetDrop`)
      (goto _label_3 :!via `Stop`))))

(event `PlayTargetDrop`
  (if (not (`self.IsDown`))
    (set `self.IsDown` true)
    (if (`self.IsDown`) :!label _label
      (`KismetSystemLibrary.Delay` (`self.ResetTime`))
      (set `self.Health` (`self.MaxHealth`))
      (`SkeletalMeshComponent.PlayAnimation` (`self.Target`) "/Game/AnimStarterPack/Idle_Rifle_Hip.Idle_Rifle_Hip" true)
      (`self.RaiseTarget`))))

(event `self.ReceiveBeginPlay`)

(event `RaiseTarget`
  (if (`self.IsDown`)
    (set `self.IsDown` false)
    (goto _label)))

(event `OnActive`
  (`SkeletalMeshComponent.PlayAnimation` (`self.Target`) "/Game/AnimStarterPack/Idle_Rifle_Hip.Idle_Rifle_Hip" true :!label _label_2)
  (if (not (`self.IsDown`))
    (`KismetSystemLibrary.MoveComponentTo` (`self.SM_Floor_A1`) (`SceneComponent.RelativeLocation` (`self.PosB`)) (struct) false false (`self.MovingTime`) :!label _label_3)
    (if (not (`self.IsDown`))
      (`KismetSystemLibrary.Delay` 0.01)
      (`KismetSystemLibrary.MoveComponentTo` (`self.SM_Floor_A1`) (`SceneComponent.RelativeLocation` (`self.PosA`)) (struct) false false (`self.MovingTime`))
      (`KismetSystemLibrary.Delay` 0.01)
      (goto _label_2))))

(fn `UpdateScore`
  (params (Score :type Integer)))

(fn `UserConstructionScript`)