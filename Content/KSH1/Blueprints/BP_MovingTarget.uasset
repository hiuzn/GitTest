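; Shooting target that slides back and forth and awards the player score when hit by a player bullet.
; After a random startup delay, two timelines loop it between its start point and a fixed X position.
; A bullet overlap on Body1 plays a death animation and adds multiplied score through the player character.
; Two seconds later it returns to idle, can be hit again and restarts its forward movement.
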(event `self.Body1.OnComponentBeginOverlap`
  (params (OverlappedComponent :type "PrimitiveComponent Object Reference") (OtherActor :type "Actor Object Reference") (OtherComp :type "PrimitiveComponent Object Reference") (OtherBodyIndex :type Integer) (bFromSweep :type Boolean) (SweepResult :type "HitResult Structure (by ref)"))
  ;[1 1 1] 타겟 죽었을 때 스코어 획득
  (cast `/Game/KSH1/Blueprints/BP_Bullet_Player` OtherActor)
  (if (not (`self.IsDead`))
    (`SkeletalMeshComponent.PlayAnimation` (`self.SkeletalMesh`) "/Game/AnimStarterPack/Death_1.Death_1" false)
    (`self.TargetDead`)
    (`self.AddScore` 1)))

(event `self.ReceiveBeginPlay`
  (bind (_returnvalue_x _returnvalue_y _returnvalue_z) (`KismetMathLibrary.BreakVector` (`self.K2_GetActorLocation`)))
  (`|ExecutionSequence`
    (:`then_0`
      (`SkeletalMeshComponent.PlayAnimation` (`self.SkeletalMesh`) "/Game/AnimStarterPack/Idle_Rifle_Hip.Idle_Rifle_Hip" false)
      (`KismetSystemLibrary.Delay` (`KismetMathLibrary.RandomFloatInRange` 0.0 10.0))
      (`|ExecutionSequence`
        (:`then_0`
          (set `self.Start` (`KismetMathLibrary.MakeVector` _returnvalue_x _returnvalue_y _returnvalue_z))
          (set `self.End` (`KismetMathLibrary.MakeVector` -1500.0 _returnvalue_y _returnvalue_z))
          (bind _asbp_third_person_character (cast `/Game/ThirdPerson/Blueprints/BP_ThirdPersonCharacter` (`GameplayStatics.GetPlayerCharacter` 0)))
          (set `self.Char Ref` _asbp_third_person_character)
          (bind (_direction `_새_트랙_0`) (`Timeline|Move` :!via `PlayFromStart` :!label _label)
            (:`Update`
              (`self.K2_SetActorRelativeLocation` (`KismetMathLibrary.VLerp` (`self.Start`) (`self.End`) `_새_트랙_0`)))
            (:`Finished`
              (`KismetSystemLibrary.Delay` 0.2)
              (bind (_direction_2 `_새_트랙_0_2`) (`Timeline|Move Back` :!via `ReverseFromEnd`)
                (:`Update`
                  (`self.K2_SetActorRelativeLocation` (`KismetMathLibrary.VLerp` (`self.Start`) (`self.End`) `_새_트랙_0_2`)))
                (:`Finished`
                  (goto _label :!via `PlayFromStart`))))))))))

(event `TargetDead`
  ;[1 1 1] 타겟 다운
  (set `self.IsDead` true)
  (if (`self.IsDead`)
    (`KismetSystemLibrary.Delay` 2.0)
    (`SkeletalMeshComponent.PlayAnimation` (`self.SkeletalMesh`) "/Game/AnimStarterPack/Idle_Rifle_Hip.Idle_Rifle_Hip" false)
    (set `self.IsDead` false)
    (goto _label :!via `PlayFromStart`)))

(event `CustomEvent_3`
  ;[1 1 1] 타겟 다운
  (set `self.IsDead` true)
  (if (`self.IsDead`)
    (`KismetSystemLibrary.Delay` 2.0)
    (`SkeletalMeshComponent.PlayAnimation` (`self.SkeletalMesh`) "/Game/AnimStarterPack/Idle_Rifle_Hip.Idle_Rifle_Hip" false)
    (set `self.IsDead` false)))

(fn `AddScore`
  (params (Score :type Integer))
  (bind _asbp_third_person_character (cast `/Game/ThirdPerson/Blueprints/BP_ThirdPersonCharacter` (`GameplayStatics.GetPlayerPawn` 0)))
  (`/Game/ThirdPerson/Blueprints/BP_ThirdPersonCharacter.AddScore` _asbp_third_person_character (* Score (`self.Multiflier`))))

(fn `UserConstructionScript`)