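; Rifle-armed enemy AI character that chases the player, shoots and dies when its health runs out.
; From BeginPlay it loops AIMoveTo on the player controller into a montage attack, line-tracing from the muzzle socket (end point not offset by start) to apply damage.
; Pawn sensing snaps it toward a seen player character and sets walk speed.
; Damage reduces health until death sets IsDead, stops movement and plays a montage.
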(event `self.PawnSensing.OnSeePawn`
  (params (Pawn :type "Pawn Object Reference"))
  (cast `/Game/ThirdPerson/Blueprints/BP_ThirdPersonCharacter` Pawn)
  (`self.K2_SetActorRotation` (`KismetMathLibrary.FindLookAtRotation` (`self.K2_GetActorLocation`) (`self.K2_GetActorLocation` Pawn)))
  (set `CharacterMovementComponent.MaxWalkSpeed` 360.0 (`self.CharacterMovement`)))

(event `self.ReceiveBeginPlay`
  (`self.RunToPlayer`))

(event `RunToPlayer`
  (if (not (`self.IsDead`))
    (`|AIMoveTo` self (0.0 0.0 0.0) (`GameplayStatics.GetPlayerController` 0) 250.0
      (:`OnSuccess`
        (`self.AttackPlayer`))
      (:`OnFail`
        (`self.RunToPlayer`)))))

(event `AttackPlayer`
  (bind _weapons (`self.Weapons`))
  (bind (_returnvalue_location _returnvalue_rotation) (`KismetMathLibrary.BreakTransform` (`SceneComponent.GetSocketTransform` _weapons "MuzzleFlash" "RTS_World")))
  (`|PlayMontage` (`self.Mesh`) "/Game/Characters/AI_Enemy/Animations/AI_Fire_Rifle_Hip_Montage.AI_Fire_Rifle_Hip_Montage"
    (:`then`
      (`SkeletalMeshComponent.PlayAnimation` _weapons "/Game/MilitaryWeapDark/Weapons/Anims/Fire_Rifle_W.Fire_Rifle_W" false)
      (bind (_outhit _returnvalue) (`KismetSystemLibrary.LineTraceSingle` _returnvalue_location (* (`KismetMathLibrary.GetForwardVector` _returnvalue_rotation) 15000.0) "TraceTypeQuery2"))
      (if _returnvalue
        (`GameplayStatics.ApplyDamage` (`.HitActor` (`GameplayStatics.BreakHitResult` _outhit)) 1.0 null null "/Script/Engine.DamageType")))
    (:`OnCompleted`
      (`self.RunToPlayer`))))

(event `self.ReceiveAnyDamage`
  (params (Damage :type "Float (single-precision)") (DamageType :type "DamageType Object Reference") (InstigatedBy :type "Controller Object Reference") (DamageCauser :type "Actor Object Reference"))
  (if (`self.IsDead`)
    _
    (elif (<= (`self.Health`) 0.0)
      (`self.AIDeath`)
      (else
        (bind _output_get (set `self.Health` (- (`self.Health`) Damage)))
        (`KismetSystemLibrary.PrintString` (`KismetStringLibrary.Conv_DoubleToString` _output_get))
        (if (<= _output_get 0.0)
          (`self.AIDeath`))))))

(event `AIDeath`
  (set `self.IsDead` true)
  (`MovementComponent.StopMovementImmediately` (`self.CharacterMovement`))
  (`|PlayMontage` (`self.Mesh`) "/Game/Characters/AI_Enemy/Animations/AI_Death_1_Montage.AI_Death_1_Montage"))

(fn `UserConstructionScript`)