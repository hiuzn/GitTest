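; Zombie enemy character that chases the player once within 500 units, attacks with a kick and dies from damage.
; Tick checks distance until the player is found, then AIMoveTo targets the player controller and loops with the attack montage.
; The montage notify runs a sphere overlap at an arrow component to damage the player character.
; Pawn sensing sets walk speed, while damage drains Health until death stops movement and plays a dying montage.
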(event `self.ReceiveTick`
  (params (DeltaSeconds :type "Float (single-precision)"))
  (if (`self.Find`)
    _
    (elif (not (`self.IsDead`))
      (`self.RuntoPlayer`))))

(event `self.ReceiveBeginPlay`)

(event `RunToPlayer`
  (if (or (<= (`KismetMathLibrary.VSize` (- (`SceneComponent.K2_GetComponentLocation` (`self.Mesh`)) (`PlayerController.GetFocalLocation` (`GameplayStatics.GetPlayerController` 0)))) 500.0) (`self.Find`))
    (if (not (`self.IsDead`))
      (set `self.Find` true)
      (`|AIMoveTo` self (0.0 0.0 0.0) (`GameplayStatics.GetPlayerController` 0) 100.0
        (:`OnSuccess`
          (`self.Attack Player`))
        (:`OnFail`
          (`self.RunToPlayer`))))))

(event `self.PawnSensing.OnSeePawn`
  (params (Pawn :type "Pawn Object Reference"))
  (set `CharacterMovementComponent.MaxWalkSpeed` 360.0 (`self.CharacterMovement`)))

(event `Attack Player`
  (`|PlayMontage` (`self.Mesh`) "/Game/Characters/Zombies/ManZombie/Animation/zombie_Kicking_Montage.zombie_Kicking_Montage"
    (:`OnCompleted`
      (`self.RunToPlayer`))
    (:`OnNotifyBegin`
      (bind (_outactors _returnvalue) (`KismetSystemLibrary.SphereOverlapActors` (`SceneComponent.K2_GetComponentLocation` (`self.Arrow1`)) 200.0 (`|MakeArray` "ObjectTypeQuery3" :!type "EObjectTypeQuery Enum") "/Game/ThirdPerson/Blueprints/BP_ThirdPersonCharacter.BP_ThirdPersonCharacter_C" (`|MakeArray` self :!type "Actor Object Reference")))
      (if _returnvalue
        (for _array_element _outactors
          (`GameplayStatics.ApplyDamage` _array_element 20.0 (`self.GetController`) self "/Script/Engine.DamageType"))))))

(event `self.ReceiveAnyDamage`
  (params (Damage :type "Float (single-precision)") (DamageType :type "DamageType Object Reference") (InstigatedBy :type "Controller Object Reference") (DamageCauser :type "Actor Object Reference"))
  (if (`self.IsDead`)
    _
    (elif (<= (`self.Health`) 0.0)
      (`self.Death`)
      (else
        (bind _output_get (set `self.Health` (- (`self.Health`) Damage)))
        (if (<= _output_get 0.0)
          (`self.Death`))))))

(event `Death`
  (set `self.IsDead` true)
  (`MovementComponent.StopMovementImmediately` (`self.CharacterMovement`))
  (`|PlayMontage` (`self.Mesh`) "/Game/Characters/Zombies/ManZombie/Animation/Zombie_Dying_Anim_Montage.Zombie_Dying_Anim_Montage"))

(event `self.Mesh.OnComponentHit`
  (params (HitComponent :type "PrimitiveComponent Object Reference") (OtherActor :type "Actor Object Reference") (OtherComp :type "PrimitiveComponent Object Reference") (NormalImpulse :type "Vector Structure") (Hit :type "HitResult Structure (by ref)")))

(fn `UserConstructionScript`)