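; Zombie girl enemy that chases and melee-attacks the player, starting once the player controller's focal location is within 500 units.
; Tick polls until that range check latches Find, then AI MoveTo and the attack montage loop, retrying on failed moves; seeing a pawn sets walk speed.
; A montage notify triggers a sphere-overlap hit at Arrow1.
; Damage reduces health, playing a death montage or a hit reaction that also loosens collision without restoring it.
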(event `self.ReceiveBeginPlay`)

(event `self.ReceiveTick`
  (params (DeltaSeconds :type "Float (single-precision)"))
  (if (`self.Find`)
    _
    (elif (not (`self.IsDead`))
      (`self.RuntoPlayer`))))

(event `RuntoPlayer`
  (if (or (<= (`KismetMathLibrary.VSize` (- (`SceneComponent.K2_GetComponentLocation` (`self.Mesh`)) (`PlayerController.GetFocalLocation` (`GameplayStatics.GetPlayerController` 0)))) 500.0) (`self.Find`))
    (if (not (`self.IsDead`))
      (set `self.Find` true)
      (`|AIMoveTo` self (0.0 0.0 0.0) (`GameplayStatics.GetPlayerController` 0) 100.0
        (:`OnSuccess`
          (`self.AttackPlayer`))
        (:`OnFail`
          (`self.RuntoPlayer`))))))

(event `self.PawnSensing.OnSeePawn`
  (params (Pawn :type "Pawn Object Reference"))
  (set `CharacterMovementComponent.MaxWalkSpeed` 360.0 (`self.CharacterMovement`)))

(event `AttackPlayer`
  (`|PlayMontage` (`self.Mesh`) "/Game/Characters/Zombies/WomanZombie/Animations/zombie_attack_Montage.zombie_attack_Montage"
    (:`OnCompleted`
      (`self.RuntoPlayer`))
    (:`OnNotifyBegin`
      (bind (_outactors _returnvalue) (`KismetSystemLibrary.SphereOverlapActors` (`SceneComponent.K2_GetComponentLocation` (`self.Arrow1`)) 80.0 (`|MakeArray` "ObjectTypeQuery3" :!type "EObjectTypeQuery Enum") "/Game/ThirdPerson/Blueprints/BP_ThirdPersonCharacter.BP_ThirdPersonCharacter_C" (`|MakeArray` self :!type "Actor Object Reference")))
      (if _returnvalue
        (for _array_element _outactors
          (`GameplayStatics.ApplyDamage` _array_element 20.0 (`self.GetController`) self "/Script/Engine.DamageType"))))))

(event `self.ReceiveAnyDamage`
  (params (Damage :type "Float (single-precision)") (DamageType :type "DamageType Object Reference") (InstigatedBy :type "Controller Object Reference") (DamageCauser :type "Actor Object Reference"))
  (if (`self.IsDead`)
    _
    (elif (<= (`self.Health`) 0.0)
      (`self.Death`)
      (else
        (bind _output_get (set `self.Health` (- (`self.Health`) Damage)))
        (`KismetSystemLibrary.PrintString` (`KismetStringLibrary.Conv_DoubleToString` _output_get))
        (if (<= _output_get 0.0)
          (`self.Death`)
          (else
            (`|PlayMontage` (`self.Mesh`) "/Game/Characters/Zombies/WomanZombie/Animations/Zombie_Reaction_Hit_mixamo_com_Montage.Zombie_Reaction_Hit_mixamo_com_Montage"
              (:`then`
                (`PrimitiveComponent.SetCollisionResponseToChannel` (`self.CapsuleComponent`) "ECC_Pawn" "ECR_Overlap")
                (`PrimitiveComponent.SetCollisionEnabled` (`self.Mesh`) "NoCollision")))))))))

(event `Death`
  (set `self.IsDead` true)
  (`MovementComponent.StopMovementImmediately` (`self.CharacterMovement`))
  (`|PlayMontage` (`self.Mesh`) "/Game/Characters/Zombies/WomanZombie/Animations/zombie_dying_Montage.zombie_dying_Montage"))

(fn `UserConstructionScript`)