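; Boss enemy character that plays an entrance animation, then acts and takes damage only once IsAppear is set.
; BeginPlay starts a chase-attack loop if already appeared: AIMoveTo the player controller, then a rifle montage with a muzzle line trace applying damage.
; Pawn sensing turns it toward the seen player and sets walk speed.
; Damage reduces Health, and at zero it stops movement and plays a death montage.
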(event `AppearScene`
  (`KismetSystemLibrary.PrintText` "\"APPEAR SCENE에 들어왔습니다.\"" true true (struct :`G` 0.66 :`B` 1.0 :`A` 1.0) 5.0)
  (`SkeletalMeshComponent.PlayAnimation` (`self.Mesh`) "/Game/Characters/Boss/Animations/BS_Boss_Appear_Scene.BS_Boss_Appear_Scene" false)
  (`KismetSystemLibrary.PrintText` "\"애니메이션이 플레이 되었습니다\"" true true (struct :`G` 0.66 :`B` 1.0 :`A` 1.0) 5.0)
  (set `self.IsAppear` true))

(event `self.ReceiveBeginPlay`
  (if (`self.IsAppear`)
    (`self.RunToPlayer`)))

(event `self.PawnSensing.OnSeePawn`
  (params (Pawn :type "Pawn Object Reference"))
  (if (`self.IsAppear`)
    (if (not (`self.IsDead`))
      (cast `/Game/ThirdPerson/Blueprints/BP_ThirdPersonCharacter` Pawn)
      (`self.K2_SetActorRotation` (`KismetMathLibrary.FindLookAtRotation` (`self.K2_GetActorLocation`) (`self.K2_GetActorLocation` Pawn)))
      (set `CharacterMovementComponent.MaxWalkSpeed` 360.0 (`self.CharacterMovement`)))))

(event `RunToPlayer`
  (if (`self.IsAppear`)
    (if (not (`self.IsDead`))
      (`|AIMoveTo` self (0.0 0.0 0.0) (`GameplayStatics.GetPlayerController` 0) 250.0
        (:`OnSuccess`
          (`self.AttackPlayer`))
        (:`OnFail`
          (`self.RunToPlayer`))))))

(event `AttackPlayer`
  (bind _weapons (`self.Weapons`))
  (bind (_returnvalue_location _returnvalue_rotation) (`KismetMathLibrary.BreakTransform` (`SceneComponent.GetSocketTransform` _weapons "MuzzleFlash" "RTS_World")))
  (`|PlayMontage` (`self.Mesh`) "/Game/Characters/Boss/Animations/Firing_Rifle_Boss_Montage.Firing_Rifle_Boss_Montage"
    (:`then`
      (`SkeletalMeshComponent.PlayAnimation` _weapons "/Game/MilitaryWeapDark/Weapons/Anims/Fire_Rifle_W.Fire_Rifle_W" false)
      (bind (_outhit _returnvalue) (`KismetSystemLibrary.LineTraceSingle` _returnvalue_location (* (`KismetMathLibrary.GetForwardVector` _returnvalue_rotation) 15000.0) "TraceTypeQuery2"))
      (if _returnvalue
        (`GameplayStatics.ApplyDamage` (`.HitActor` (`GameplayStatics.BreakHitResult` _outhit)) 1.0 null null "/Script/Engine.DamageType")))
    (:`OnCompleted`
      (`self.RunToPlayer`))))

(event `self.ReceiveAnyDamage`
  (params (Damage :type "Float (single-precision)") (DamageType :type "DamageType Object Reference") (InstigatedBy :type "Controller Object Reference") (DamageCauser :type "Actor Object Reference"))
  (if (`self.IsAppear`)
    (if (`self.IsDead`)
      _
      (elif (<= (`self.Health`) 0.0)
        (`self.AIDeath`)
        (else
          (bind _output_get (set `self.Health` (- (`self.Health`) Damage)))
          (`KismetSystemLibrary.PrintText` (`KismetTextLibrary.Conv_StringToText` (`KismetStringLibrary.Concat_StrStr` "<-----남아있는 hp: " (`KismetStringLibrary.Conv_DoubleToString` _output_get) "입니다----->")))
          (if (<= _output_get 0.0)
            (`self.AIDeath`)))))))

(event `AIDeath`
  (set `self.IsDead` true)
  (`MovementComponent.StopMovementImmediately` (`self.CharacterMovement`))
  (`|PlayMontage` (`self.Mesh`) "/Game/Characters/Boss/Animations/Mutant_Dying_Boss_Montage.Mutant_Dying_Boss_Montage"))

(fn `UserConstructionScript`)